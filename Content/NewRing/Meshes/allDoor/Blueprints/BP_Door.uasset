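; BP_Door is a VR door that the player swings open by grabbing it from the front or back.
; A grab stores the motion controller and starts a fast looping timer running UpdateRotation; dropping clears both.
; UpdateRotation converts the controller position into RotateOrigin's local space, adds its look-at yaw to the hinge's yaw, and clamps the result to a quarter-turn swing.
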(event OnGrabbed(FrontGrab)
  (params (Motion%20Controller :type Motion%20Controller%20Component%20Object%20Reference))
  (Variables|Default|SetMotion%20Controller Motion%20Controller)
  (bind _returnvalue (Utilities|Time|SetTimerbyFunctionName 0 "UpdateRotation" 0.01 true))
  (Variables|Default|SetTimer _returnvalue))

(event OnDropped(FrontGrab)
  (Utilities|Time|ClearandInvalidateTimerbyHandle (Variables|Default|GetTimer))
  (Variables|Default|SetMotion%20Controller 0))

(event OnGrabbed(BackGrab)
  (params (Motion%20Controller :type Motion%20Controller%20Component%20Object%20Reference))
  (Variables|Default|SetMotion%20Controller Motion%20Controller)
  (bind _returnvalue (Utilities|Time|SetTimerbyFunctionName 0 "UpdateRotation" 0.01 true))
  (Variables|Default|SetTimer _returnvalue))

(event OnDropped(BackGrab)
  (Utilities|Time|ClearandInvalidateTimerbyHandle (Variables|Default|GetTimer))
  (Variables|Default|SetMotion%20Controller 0))

(fn ConstructionScript)

(fn UpdateRotation
  (bind _rotateorigin (Variables|Default|GetRotateOrigin))
  (bind _rotateorigin_2 (Variables|Default|GetRotateOrigin))
  (bind _returnvalue (Transformation|GetWorldTransform _rotateorigin))
  (bind _relativerotation (Variables|/Script/Engine.SceneComponent|GetRelativeRotation _rotateorigin_2))
  (Transformation|SetRelativeRotation _rotateorigin_2 (Math|Rotator|MakeRotator (.roll _relativerotation) (.pitch _relativerotation) (Math|Float|Clamp(Float) (+ (.yaw _relativerotation) (.yaw (Math|Rotator|FindLookatRotation (Math|Vector|MakeVector 0.0 0.0 0.0) (.location (Math|Transform|MakeRelativeTransform (Transformation|GetWorldTransform (Variables|Default|GetMotion%20Controller)) (Math|Transform|MakeTransform (.location _returnvalue) (.rotation _returnvalue) (.scale _returnvalue))))))) 0.0 9e+01)) false false))